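; Side-view sword enemy with flipbook animation that lunges at the player and deals damage on hit to actors tagged "player".
; Tick runs a cooldown timer that, while the player is in range, triggers capsule impulses along X toward them, scaled by distance.
; Tick also flips the sprite and picks idle, run, run-attack or death flipbooks from velocity, distance and health.
; Incoming damage lowers health, destroying the actor shortly after death.
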(event `aimove to`)

(event `self.ReceiveHit`
  (params (MyComp :type "PrimitiveComponent Object Reference") (Other :type "Actor Object Reference") (OtherComp :type "PrimitiveComponent Object Reference") (bSelfMoved :type Boolean) (HitLocation :type "Vector Structure") (HitNormal :type "Vector Structure") (NormalImpulse :type "Vector Structure") (Hit :type "HitResult Structure (by ref)"))
  ;[1 1 1] apply damage
  (if (and (`self.ActorHasTag` Other "player") (not (<= (stale `self.ReceiveAnyDamage` _output_get) 0.0)))
    (`GameplayStatics.ApplyDamage` Other (`self.dmg`))))

(event `self.ReceiveTick`
  (params (DeltaSeconds :type "Float (single-precision)"))
  (bind _returnvalue (`GameplayStatics.GetPlayerPawn` 0))
  (set `self.dt` DeltaSeconds)
  (set `self.PlayerD` (`KismetMathLibrary.Conv_DoubleToVector` (`self.GetDistanceTo` (`GameplayStatics.GetPlayerPawn` 0))))
  (set `self.pd` (`self.GetDistanceTo` _returnvalue))
  (`|ExecutionSequence`
    (:`then_0`
      (bind _returnvalue_2 (not (<= (stale `self.ReceiveAnyDamage` _output_get) 0.0)))
      (if _returnvalue_2
        ;[1 1 1] reset timer
        (if (<= (`self.reset_tmr`) 0.0)
          (if (<= (`self.pd`) 1000.0)
            (set `self.reset_tmr` (`self.reset`)))
          (else
            (set `self.reset_tmr` (- (`self.reset_tmr`) (`self.dt`)))))))
    (:`then_1`
      (if _returnvalue_2
        (`|ExecutionSequence`
          (:`then_1`
            (if (and (<= (`self.pd`) 1000.0) (== (`self.reset_tmr`) (`self.reset`)))
              (if (> (.x (`self.K2_GetActorLocation` _returnvalue)) (.x (`self.K2_GetActorLocation`)))
                (set `self.xk` 1.0)
                (else
                  (set `self.xk` -1.0)))
              (`|ExecutionSequence`
                (:`then_0`
                  (`PrimitiveComponent.AddImpulse` (`self.CapsuleComponent`) (`KismetMathLibrary.MakeVector` (* (.x (`self.PlayerD`)) (`self.xk`) (`self.spd_x`))) "None" false))))))))
    (:`then_2`
      (`|ExecutionSequence`
        (:`then_0`
          ;[1 1 1] rotationFlipbook
          (if (< (`self.xk`) 0.0)
            (`SceneComponent.K2_SetWorldRotation` :`self` (`self.Flipbook`))
            (else
              (`SceneComponent.K2_SetWorldRotation` (`self.Flipbook`) (struct :`Yaw` 180.0) false false))))
        (:`then_1`
          (if (> (`KismetMathLibrary.VSize` (`self.GetVelocity`)) 0.0)
            (if (<= (`self.pd`) 150.0)
              (set `self.Fb_Anim` "/Game/spite_for_animation/Enemyswordrunatack1.Enemyswordrunatack1")
              (else
                (set `self.Fb_Anim` "/Game/spite_for_animation/enmyrunsword.enmyrunsword")))
            (else
              (set `self.Fb_Anim` "/Game/spite_for_animation/enemysword1.enemysword1"))))
        (:`then_2`
          (if (<= (`self.hp`) 0.0)
            (set `self.Fb_Anim` "/Game/spite_for_animation/enemysworddie2.enemysworddie2")))
        (:`then_3`
          ;[1 1 1] set flipbook
          (`PaperFlipbookComponent.SetFlipbook` (`self.Flipbook`) (`self.Fb_Anim`)))))
    (:`then_3`)))

(event `self.ReceiveAnyDamage`
  (params (Damage :type "Float (single-precision)") (DamageType :type "DamageType Object Reference") (InstigatedBy :type "Controller Object Reference") (DamageCauser :type "Actor Object Reference"))
  ;[1 1 1] Actor destroy
  (bind _output_get (set `self.hp` (- (`self.hp`) Damage)))
  (if (<= _output_get 0.0)
    (`|ExecutionSequence`
      (:`then_0`
        (`KismetSystemLibrary.Delay` 0.8)
        (`self.K2_DestroyActor`)))))

(event `self.FloatingPawnMovement.OnComponentActivated`
  (params (Component :type "ActorComponent Object Reference") (bReset :type Boolean)))

(fn `UserConstructionScript`
  (`parent.UserConstructionScript`))