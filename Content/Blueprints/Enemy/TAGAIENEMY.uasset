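; Side-scroller sword enemy pawn that chases the player, damages player-tagged actors it hits while alive, and drops a coin on death.
; Pawn sensing starts AI MoveTo on the player, falling back to a right-then-left patrol between tagged actors.
; Tick picks the flipbook from speed, player distance and health, and flips facing.
; The Dead flag is inverted: true means alive.
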(event `Move`
  (params (Direction :type "Vector Structure") (Scale :type "Float (double-precision)"))
  (`self.AddMovementInput` Direction Scale))

(event `self.ReceiveHit`
  (params (MyComp :type "PrimitiveComponent Object Reference") (Other :type "Actor Object Reference") (OtherComp :type "PrimitiveComponent Object Reference") (bSelfMoved :type Boolean) (HitLocation :type "Vector Structure") (HitNormal :type "Vector Structure") (NormalImpulse :type "Vector Structure") (Hit :type "HitResult Structure (by ref)"))
  ;[1 1 1] apply damage
  (if (`self.dead`)
    (if (`self.ActorHasTag` Other "player")
      (`GameplayStatics.ApplyDamage` Other (`self.dmg`)))))

(event `self.ReceiveTick`
  (params (DeltaSeconds :type "Float (single-precision)"))
  (bind _returnvalue (`GameplayStatics.GetPlayerPawn` 0))
  (if (not (<= (stale `self.ReceiveAnyDamage` _output_get) 0.0))
    (set `self.dead` true)
    (else
      (set `self.dead` false)))
  (set `self.dt` DeltaSeconds)
  (set `self.pd` (`self.GetDistanceTo` _returnvalue))
  (`|ExecutionSequence`
    (:`then_0`
      (if (`self.dead`)
        ;[1 1 1] reset timer
        (if (<= (`self.reset_tmr`) 0.0)
          (if (<= (`self.pd`) 1000.0)
            (set `self.reset_tmr` (`self.reset`)))
          (else
            (set `self.reset_tmr` (- (`self.reset_tmr`) (`self.dt`)))))))
    (:`then_1`
      (if true
        (`|ExecutionSequence`
          (:`then_1`
            (if (<= (`self.pd`) 300.0)
              (if (> (.x (`self.K2_GetActorLocation` _returnvalue)) (.x (`self.K2_GetActorLocation`)))
                (set `self.xk` 1.0)
                (else
                  (set `self.xk` -1.0))))))))
    (:`then_2`
      (`|ExecutionSequence`
        (:`then_0`
          ;[1 1 1] rotationFlipbook
          (if (< (`self.xk`) 0.0)
            (`SceneComponent.K2_SetWorldRotation` :`self` (`self.Flipbook`))
            (else
              (`SceneComponent.K2_SetWorldRotation` (`self.Flipbook`) (struct :`Yaw` 180.0) false false))))
        (:`then_1`
          (if (> (`KismetMathLibrary.VSize` (`self.GetVelocity`)) 0.0)
            (if (<= (`self.pd`) 200.0)
              (set `self.Fb Anim` "/Game/spite_for_animation/Enemyswordrunatack1.Enemyswordrunatack1")
              (else
                (set `self.Fb Anim` "/Game/spite_for_animation/enmyrunsword.enmyrunsword")))
            (else
              (set `self.Fb Anim` "/Game/spite_for_animation/enemysword1.enemysword1"))))
        (:`then_2`
          (if (<= (`self.hp`) 0.0)
            (set `self.Fb Anim` "/Game/spite_for_animation/enemysworddie2.enemysworddie2")))
        (:`then_3`
          ;[1 1 1] set flipbook
          (`PaperFlipbookComponent.SetFlipbook` (`self.Flipbook`) (`self.Fb Anim`)))))))

(event `self.ReceiveAnyDamage`
  (params (Damage :type "Float (single-precision)") (DamageType :type "DamageType Object Reference") (InstigatedBy :type "Controller Object Reference") (DamageCauser :type "Actor Object Reference"))
  ;[1 1 1] Actor destroy
  (bind _output_get (set `self.hp` (- (`self.hp`) Damage)))
  (if (<= _output_get 0.0)
    (`|ExecutionSequence`
      (:`then_0`
        (`KismetSystemLibrary.Delay` 0.8)
        (`self.K2_DestroyActor`)
        (`|SpawnActorFromClass` "/Game/Blueprints/coin.coin_C" (`KismetMathLibrary.MakeTransform` (`self.K2_GetActorLocation`)) "AdjustIfPossibleButDontSpawnIfColliding" "OverrideRootScale" null null)))))

(event `self.PawnSensing.OnSeePawn`
  (params (Pawn :type "Pawn Object Reference"))
  (bind _as2dside_scroller_character (cast `/Game/2DSideScrollerBP/Blueprints/2DSideScrollerCharacter` Pawn :!label _label)
    (:`then`
      (`|AIMoveTo` self (0.0 0.0 0.0) _as2dside_scroller_character
        (:`OnFail`
          _)))
    (:`CastFailed`
      _))
  (`|ExecutionSequence`
    (:`then_0`
      (bind _target (`self.FindTargetByTag` "right"))
      (`|AIMoveTo` self (0.0 0.0 0.0) _target 10.0 true
        (:`OnSuccess`
          (`KismetSystemLibrary.Delay` 1.0)
          (bind _target_2 (`self.FindTargetByTag` "left"))
          (`|AIMoveTo` self (0.0 0.0 0.0) _target_2 10.0 true
            (:`OnSuccess`
              (`KismetSystemLibrary.Delay` 1.0)
              (goto _label))))))))

(fn `FindTargetByTag`
  (params (Tag :type Name))
  (returns (Target :type "Actor Object Reference"))
  (locals (L_target :type "Actor Object Reference"))
  (bind _outactors (`GameplayStatics.GetAllActorsOfClass` "/Script/Engine.Actor"))
  (for _array_element _outactors
    (if (`self.ActorHasTag` _array_element Tag)
      (set `local.L_target` _array_element)
      (break)))
  (return (`local.L_target`)))

(fn `UserConstructionScript`)