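; Coin pickup actor for a 2D side-scroller that adds one to the player character's Money when touched.
; On overlap it casts the other actor to 2DSideScrollerCharacter, destroys itself, then computes the new total, prints it and writes it back to the character.
; Tick, BeginPlay and the construction script are empty.
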(event `self.ReceiveTick`
  (params (DeltaSeconds :type "Float (single-precision)")))

(event `self.ReceiveBeginPlay`)

(event `self.ReceiveActorBeginOverlap`
  (params (OtherActor :type "Actor Object Reference"))
  (bind _as2dside_scroller_character (cast `/Game/2DSideScrollerBP/Blueprints/2DSideScrollerCharacter` OtherActor))
  (`self.K2_DestroyActor`)
  (`|ExecutionSequence`
    (:`then_0`
      (bind _output_get (set `self.moneyUp` (+ (`/Game/2DSideScrollerBP/Blueprints/2DSideScrollerCharacter.money` _as2dside_scroller_character) 1)))
      (set `self.moneyt` (`KismetStringLibrary.Conv_IntToString` _output_get)))
    (:`then_1`
      (`KismetSystemLibrary.PrintString` (`KismetStringLibrary.Conv_IntToString` _output_get))
      (set `/Game/2DSideScrollerBP/Blueprints/2DSideScrollerCharacter.money` _output_get _as2dside_scroller_character))))

(fn `UserConstructionScript`)